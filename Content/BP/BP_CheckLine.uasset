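; BP_CheckLine is an actor that clears completed lines of BP_SingleBlock actors in a falling-block, Tetris-style game.
; CheckLine treats each box component as a row sensor, full at ten overlapping blocks, and adds to DropAmount per full row.
; Full rows below the current CutOffLineZ lower that cutoff and have their blocks destroyed with particle effects.
; Blocks above the cutoff then get TargetZ reduced by DropAmount, neither value being reset here.
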(fn `CheckLine`
  (locals (`Overlapping Actors` :type "Array of Actor Object Reference") (DropAmount :type "Float (double-precision)") (CutOffLineZ :type "Float (double-precision)" :default 2000.0))
  (for _array_element (`self.K2_GetComponentsByClass` "/Script/Engine.BoxComponent")
    (set `local.Overlapping Actors` (`PrimitiveComponent.GetOverlappingActors` _array_element "/Game/BP/BP_SingleBlock.BP_SingleBlock_C"))
    (if (== (`KismetArrayLibrary.Array_Length` (`local.Overlapping Actors`)) 10)
      (set `local.DropAmount` (+ (`local.DropAmount`) 50.0))
      (bind (_returnvalue_x _returnvalue_y _returnvalue_z) (`KismetMathLibrary.BreakVector` (`SceneComponent.K2_GetComponentLocation` _array_element)))
      (if (< _returnvalue_z (`local.CutOffLineZ`))
        (set `local.CutOffLineZ` _returnvalue_z)
        (for _array_element_2 (`local.Overlapping Actors`)
          (`GameplayStatics.SpawnEmitterAtLocation` null (`self.K2_GetActorLocation` _array_element_2) (struct) (0.5 0.5 0.5))
          (`self.K2_DestroyActor` _array_element_2)))))
  (bind _outactors (`GameplayStatics.GetAllActorsOfClass` "/Game/BP/BP_SingleBlock.BP_SingleBlock_C"))
  (for _array_element_3 _outactors
    (bind (_returnvalue_x_2 _returnvalue_y_2 _returnvalue_z_2) (`KismetMathLibrary.BreakVector` (`self.K2_GetActorLocation` _array_element_3)))
    (if (> _returnvalue_z_2 (`local.CutOffLineZ`))
      (set `/Game/BP/BP_SingleBlock.TargetZ` (- (`/Game/BP/BP_SingleBlock.TargetZ` _array_element_3) (`local.DropAmount`)) _array_element_3))))

(fn `UserConstructionScript`)